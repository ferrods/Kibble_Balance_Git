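; BP_Laptop is a calibration laptop actor that displays light spot readings in the game.
; Its PopulateLaptop event takes an array and loops over it, converting the first four elements to text.
; Each element is written by index to its own LightSpotValue text component, and any further entries are ignored.
; It has no other active logic, as the default events and construction script are empty.
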(event Custom|PopulateLaptop
  (params (Array :type Array%20of%20Strings))
  (for (_array_element _array_index) Array
    (if (== _array_index 0)
      (Rendering|Components|TextRender|SetText (Variables|Default|GetLightSpotValue_1) (Utilities|Text|ToText(String) _array_element))
      (elif (== _array_index 1)
        (Rendering|Components|TextRender|SetText (Variables|Default|GetLightSpotValue_2) (Utilities|Text|ToText(String) _array_element))
        (elif (== _array_index 2)
          (Rendering|Components|TextRender|SetText (Variables|Default|GetLightSpotValue_3) (Utilities|Text|ToText(String) _array_element))
          (elif (== _array_index 3)
            (Rendering|Components|TextRender|SetText (Variables|Default|GetLightSpotValue_4) (Utilities|Text|ToText(String) _array_element))))))))

(event EventBeginPlay)

(event Collision|EventActorBeginOverlap
  (params (OtherActor :type Actor%20Object%20Reference)))

(event EventTick
  (params (DeltaSeconds :type Float%20%28single-precision%29)))

(fn ConstructionScript)