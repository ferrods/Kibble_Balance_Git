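; BP_NumberPad is a calibration number pad that shows typed entries, capped at five, on its NumberScreen text.
; SetNumPad_Text stores each entry in Numbers and appends it to the display string, while BackSpace trims the last character and array element.
; After either edit, the current string is added to an ever-growing string array, which is passed to the first BP_Submit found in the level via GetLightSpotValues.
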(event Custom|SetNumPad_Text
  (params (Item :type Text))
  ;[1 1 1] Populate an Array for the Text Render
  (if (< (Utilities|Array|Length (Variables|Default|GetNumbers)) 5)
    (CallFunction|PopulateArray Item (stale Custom|IncrementCounter _countinc))
    (for _array_element (Variables|Default|GetNumbers)
      _)
    (bind _output_get (Variables|Default|SetAllText (Utilities|String|Append (Variables|Default|GetAllText) (Utilities|String|ToString(Text) _array_element))))
    (Rendering|Components|TextRender|SetText (Variables|Default|GetNumberScreen) (Utilities|Text|ToText(String) _output_get))
    ;[1 1 1] Array to sent to the laptop screen
    (bind _mystringarray (CallFunction|PopulateStringArray (Variables|Default|GetAllText)))
    (bind _outactors (Actor|GetAllActorsOfClass "/Game/Nmisa1/Blueprints/Calibration_BPs/NumberPad/BP_Submit.BP_Submit_C"))
    (Default|GetLightSpotValues (Utilities|Array|Get(acopy) _outactors) _mystringarray)))

(event Custom|IncrementCounter
  ;[1 1 1] Populate an Array for the Text Render
  (bind _countinc (CallFunction|IncreaseCounter)))

(event Custom|BackSpace
  ;[1 1 1] Delete Numbers on the Text Render
  (Rendering|Components|TextRender|SetText (Variables|Default|GetNumberScreen) (Utilities|Text|ToText(String) (Utilities|String|LeftChop (Variables|Default|GetAllText) 1)))
  (Variables|Default|SetAllText (Utilities|String|LeftChop (Variables|Default|GetAllText) 1))
  (CallFunction|RemoveArrayValue)
  ;[1 1 1] Array to sent to the laptop screen
  (bind _mystringarray (CallFunction|PopulateStringArray (Variables|Default|GetAllText)))
  (bind _outactors (Actor|GetAllActorsOfClass "/Game/Nmisa1/Blueprints/Calibration_BPs/NumberPad/BP_Submit.BP_Submit_C"))
  (Default|GetLightSpotValues (Utilities|Array|Get(acopy) _outactors) _mystringarray))

(event EventBeginPlay)

(event Collision|EventActorBeginOverlap
  (params (OtherActor :type Actor%20Object%20Reference)))

(event EventTick
  (params (DeltaSeconds :type Float%20%28single-precision%29)))

(fn ConstructionScript)

(fn IncreaseCounter
  (bind _result (Math|Integer|IncrementInt (Variables|Default|GetCount))
    (:%20%20
      (return _result))))

(fn PopulateArray
  (params (ArrayItem :type Text) (Index :type Integer))
  (Utilities|Array|Add (Variables|Default|GetNumbers) ArrayItem)
  (return))

(fn RemoveArrayValue
  (bind _numbers (Variables|Default|GetNumbers))
  (Utilities|Array|RemoveIndex _numbers (- (Utilities|Array|Length _numbers) 1))
  (return))

(fn PopulateStringArray
  (params (String :type String))
  (Utilities|Array|Add (Variables|Default|GetStringArray) String)
  (return (Variables|Default|GetStringArray)))